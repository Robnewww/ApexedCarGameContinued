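; Spline-driven track prop that repeats a mesh, likely a truss going by the asset name, along a spline and lights each segment.
; The construction script derives spacing from the mesh's X bounds plus an offset, then adds instanced meshes oriented toward the next spline point.
; Each step also adds a scene component and a static rect light at a fixed offset, rotated to match LightLocation.
; Event graph and NewFunction are empty.
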(fn `GetLocationAtIndex`
  (params (A1 :type Integer))
  (returns (ReturnValue :type "Vector Structure"))
  (return (`SplineComponent.GetLocationAtDistanceAlongSpline` (`self.Spline`) (* A1 (`self.Spacing`)) "Local")))

(fn `NewFunction`)

(fn `UserConstructionScript`
  (locals (NumberOfInstances :type Integer :default 0))
  (bind (_min _max) (break `Box` (`StaticMesh.GetBoundingBox` (`self.PlacedMesh`))))
  (`StaticMeshComponent.SetStaticMesh` (`self.InstancedStaticMesh`) (`self.PlacedMesh`))
  (bind _output_get (set `self.Spacing` (+ (.x (- _max _min)) (`self.Offset`))))
  (bind _output_get_2 (set `local.NumberOfInstances` (`KismetMathLibrary.FFloor` (/ (`SplineComponent.GetSplineLength` (`self.Spline`)) _output_get))))
  (for _index (range (+ _output_get_2 1))
    (bind _returnvalue (`self.GetLocationAtIndex` _index))
    (`InstancedStaticMeshComponent.AddInstance` (`self.InstancedStaticMesh`) (`KismetMathLibrary.MakeTransform` _returnvalue (`KismetMathLibrary.MakeRotFromX` (- (`self.GetLocationAtIndex` (+ _index 1)) _returnvalue))) false)
    (bind _returnvalue_2 (`KismetMathLibrary.MakeTransform` (+ _returnvalue (0.0 27.0 500.0)) (`SceneComponent.RelativeRotation` (`self.LightLocation`))))
    (`AddComponent|NODE_AddSceneComponent-0` :`bManualAttachment` true :`RelativeTransform` _returnvalue_2)
    (bind _returnvalue_3 (`AddComponent|NODE_AddRectLightComponent-1` :`RelativeTransform` _returnvalue_2))
    (`LocalLightComponent.SetIntensityUnits` _returnvalue_3 "Candelas")
    (`LightComponent.SetIntensity` _returnvalue_3 25.0)
    (`LocalLightComponent.SetAttenuationRadius` _returnvalue_3 1500.0)
    (`SceneComponent.SetMobility` _returnvalue_3 "Static")
    (`RectLightComponent.SetBarnDoorAngle` _returnvalue_3 45.0)
    (`RectLightComponent.SetBarnDoorLength` _returnvalue_3 10.0)))