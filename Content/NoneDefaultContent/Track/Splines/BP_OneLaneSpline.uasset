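; One-lane road spline actor that builds track geometry along its Road1 spline.
; The construction script adds a spline mesh component for each segment between neighboring spline points and attaches it to DefaultSceneRoot.
; Each segment takes its start and end position and tangent from the spline in local space, so the pieces follow the curve.
; The event graph holds no active logic.
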(fn `UserConstructionScript`
  (bind _road1 (`self.Road1`))
  (for _index (range (+ (- (`SplineComponent.GetNumberOfSplinePoints` (`self.Road1`)) 2) 1))
    (bind _returnvalue (`AddComponent|NODE_AddSplineMeshComponent-0`))
    (`SceneComponent.K2_AttachToComponent` _returnvalue (`self.DefaultSceneRoot`) "None" "KeepRelative" "KeepRelative" "KeepRelative" true)
    (bind (_location _tangent) (`SplineComponent.GetLocationAndTangentAtSplinePoint` _road1 _index "Local"))
    (bind (_location_2 _tangent_2) (`SplineComponent.GetLocationAndTangentAtSplinePoint` _road1 (+ _index 1) "Local"))
    (`SplineMeshComponent.SetStartAndEnd` _returnvalue _location _tangent _location_2 _tangent_2 true)))