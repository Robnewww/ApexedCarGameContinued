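; BP_FinishLineRefined is the finish line trigger that counts a vehicle's laps, times them and quits the game when the final lap completes.
; On overlap it starts the first lap, or advances the lap and resets checkpoints once all are passed.
; Tick accumulates lap time in BP_MainMenuGamemode.
; EndLapTime resets that time, saving any new best per track (Tokyo or Fuji) to the "Lapping" slot.
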(event `self.ReceiveTick`
  (params (DeltaSeconds :type "Float (single-precision)"))
  (bind _gamemoderef (`self.GameModeRef`))
  (if (`self.bLapStarted`)
    (set `/Game/NoneDefaultContent/BluePrints/BP_MainMenuGamemode.CurrentLapTime` (+ (`/Game/NoneDefaultContent/BluePrints/BP_MainMenuGamemode.CurrentLapTime` _gamemoderef) (`GameplayStatics.GetWorldDeltaSeconds`)) _gamemoderef)))

(event `self.ReceiveActorBeginOverlap`
  (params (OtherActor :type "Actor Object Reference"))
  (bind _asbp_vehicle (cast `/Game/NoneDefaultContent/VehicleStuff/BP_Vehicle` OtherActor))
  (set `self.VehicleRef` _asbp_vehicle)
  (if (== (`self.NumberOfCheckpoints`) (`/Game/NoneDefaultContent/VehicleStuff/BP_Vehicle.CurrentCheckpointRefined` _asbp_vehicle))
    (bind _currentlaprefined (`/Game/NoneDefaultContent/VehicleStuff/BP_Vehicle.CurrentLapRefined` _asbp_vehicle))
    (if (== (`self.NumberOfLaps`) _currentlaprefined)
      (`self.EndLapTime`)
      (`KismetSystemLibrary.QuitGame` null "Quit")
      (else
        (set `/Game/NoneDefaultContent/VehicleStuff/BP_Vehicle.CurrentLapRefined` (+ _currentlaprefined 1) _asbp_vehicle)
        (set `/Game/NoneDefaultContent/VehicleStuff/BP_Vehicle.CurrentCheckpointRefined` 0 _asbp_vehicle)
        (`self.EndLapTime`)
        (`self.StartLapTime`)))
    (elif (not (`/Game/NoneDefaultContent/VehicleStuff/BP_Vehicle.bIsLapping` _asbp_vehicle))
      (set `/Game/NoneDefaultContent/VehicleStuff/BP_Vehicle.bIsLapping` true _asbp_vehicle)
      (set `/Game/NoneDefaultContent/VehicleStuff/BP_Vehicle.CurrentLapRefined` (+ (`/Game/NoneDefaultContent/VehicleStuff/BP_Vehicle.CurrentLapRefined` _asbp_vehicle) 1) _asbp_vehicle)
      (`self.StartLapTime`))))

(event `self.ReceiveBeginPlay`
  (bind _asbp_main_menu_gamemode (cast `/Game/NoneDefaultContent/BluePrints/BP_MainMenuGamemode` (`GameplayStatics.GetGameMode`)))
  (set `self.GameModeRef` _asbp_main_menu_gamemode))

(fn `EndLapTime`
  (bind _gamemoderef (`self.GameModeRef`))
  (bind _gamemoderef_2 (`self.GameModeRef`))
  (bind _gamemoderef_3 (`self.GameModeRef`))
  (bind _bestlaptime (`/Game/NoneDefaultContent/BluePrints/BP_MainMenuGamemode.BestLapTime` _gamemoderef_2))
  (bind _savegameref (`/Game/NoneDefaultContent/BluePrints/BP_MainMenuGamemode.SaveGameRef` _gamemoderef_2))
  (if (< (`/Game/NoneDefaultContent/BluePrints/BP_MainMenuGamemode.CurrentLapTime` _gamemoderef_3) (`/Game/NoneDefaultContent/BluePrints/BP_MainMenuGamemode.BestLapTime` _gamemoderef_3))
    (set `/Game/NoneDefaultContent/BluePrints/BP_MainMenuGamemode.BestLapTime` (`/Game/NoneDefaultContent/BluePrints/BP_MainMenuGamemode.CurrentLapTime` _gamemoderef) _gamemoderef)
    (set `/Game/NoneDefaultContent/BluePrints/BP_MainMenuGamemode.CurrentLapTime` 0.0 _gamemoderef)
    (switch `string` (`KismetStringLibrary.Conv_NameToString` (`/Game/NoneDefaultContent/BluePrints/BP_MainMenuGamemode.LevelToLoad` (`self.GameModeRef`)))
      (:`TokyoBuildings`
        (set `/Game/NoneDefaultContent/CheckpointsRefined/BP_SaveGame.TokyoBestLapTime` _bestlaptime _savegameref))
      (:`MainFuji`
        (set `/Game/NoneDefaultContent/CheckpointsRefined/BP_SaveGame.FujiBestLapTime` _bestlaptime _savegameref)))
    (`GameplayStatics.SaveGameToSlot` _savegameref "Lapping")
    (else
      (set `/Game/NoneDefaultContent/BluePrints/BP_MainMenuGamemode.CurrentLapTime` 0.0 _gamemoderef))))

(fn `StartLapTime`
  (set `self.bLapStarted` true))

(fn `UserConstructionScript`)